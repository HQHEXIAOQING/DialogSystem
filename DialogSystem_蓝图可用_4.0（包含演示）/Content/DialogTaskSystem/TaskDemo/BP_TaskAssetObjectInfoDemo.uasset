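; Demo task object-info Blueprint for the dialog task system that manages an NPC through a task's lifecycle.
; Init spawns BP_DialogBeiEr at a named location, tagged "beier".
; Successful secondary task 1.1 sends it toward "OutLocation" and immediately tags the task source "NPC", without waiting for arrival.
; Task end removes that tag and destroys the pawn; secondary changes and task end print debug results.
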(event EventBlueprintInitTaskAssetObjectInfo
  (bind _returnvalue (AI|SpawnAIFromClass "/DialogSystem/TopDown/Blueprints/BP_DialogBeiEr.BP_DialogBeiEr_C" 0 (.Value (Class|TaskAssetObjectInfoBase|GetVectorfromNameId "SpawnLocation")) "0, 0, 0" false 0))
  (Utilities|Array|Add (Variables|/Script/Engine.Actor|GetTags _returnvalue) "beier")
  (Variables|Default|SetPawn_BeiEr _returnvalue))

(event EventBlueprintTaskSecondaryChanged
  (params (TaskNodeInfo :type Runtime%20Task%20Node%20Info%20Object%20Reference) (ChangedSecondaryId :type Name :default "None") (TaskResultType :type ETaskResultType%20Enum :default "None"))
  (bind _taskasset (Variables|Default|GetTaskAsset))
  (bind _tasksource (Variables|/Script/DialogSystem.TaskAsset|GetTaskSource _taskasset))
  (Development|PrintString (Utilities|String|Append (Utilities|String|ToString(Name) ChangedSecondaryId) (Utilities|String|EnumtoString TaskResultType)))
  (switch Utilities|FlowControl|Switch|SwitchonETaskResultType TaskResultType
    (:TaskSuccessful
      (switch name ChangedSecondaryId
        (:1.1
          (AI|AIMoveTo (Variables|Default|GetPawn_BeiEr) (.Value (Class|TaskAssetObjectInfoBase|GetVectorfromNameId (Variables|/Script/DialogSystem.TaskAsset|GetTaskAssetObjectInfoBase _taskasset) "OutLocation")) 0 5.0 false
            (:then
              (if (not (Actor|ActorHasTag _tasksource "NPC"))
                (Utilities|Array|Add (Variables|/Script/Engine.Actor|GetTags _tasksource) "NPC")))))))))

(event EventBlueprintTaskEnd
  (params (TaskNodeInfo :type Runtime%20Task%20End%20Node%20Info%20Object%20Reference))
  (Development|PrintString (Utilities|String|Append (Utilities|String|ToString(Text) (Variables|/Script/DialogSystem.RuntimeTaskEndNodeInfo|GetDialogEndNodeTitle TaskNodeInfo)) "：：" (Utilities|String|EnumtoString (Variables|/Script/DialogSystem.RuntimeTaskEndNodeInfo|GetTaskResult TaskNodeInfo))) true true "(R=0.000000,G=1.000000,B=0.000000,A=1.000000)")
  (Utilities|Array|RemoveItem (Variables|/Script/Engine.Actor|GetTags (Variables|/Script/DialogSystem.TaskAsset|GetTaskSource (Variables|Default|GetTaskAsset))) "NPC")
  (bind _pawn_beier (Variables|Default|GetPawn_BeiEr)
    (:then
      (Actor|DestroyActor _pawn_beier))
    (:else)))